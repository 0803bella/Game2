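; NPC Blueprint that runs a linear, voiced dialogue when the third-person character enters its sphere.
; On overlap it registers itself as the player's NPC, shows its dialogue widget and calls NextLine.
; NextLine steps through DT_NPCdialogue rows in order, setting text, playing voice audio and aligning text by speaker.
; Leaving the sphere or passing the last row clears references, removes the widget and resets the index.
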(event `self.ReceiveBeginPlay`
  (bind _returnvalue (`|CreateWidget` "/Game/Widget/W_NPCdialogue.W_NPCdialogue_C"))
  (set `self.W_Dialogue` _returnvalue))

(event `self.Sphere.OnComponentBeginOverlap`
  (params (OverlappedComponent :type "PrimitiveComponent Object Reference") (OtherActor :type "Actor Object Reference") (OtherComp :type "PrimitiveComponent Object Reference") (OtherBodyIndex :type Integer) (bFromSweep :type Boolean) (SweepResult :type "HitResult Structure (by ref)"))
  (bind _asbp_third_person_character (cast `/Game/ThirdPerson/Blueprints/BP_ThirdPersonCharacter` OtherActor))
  (bind _output_get (set `self.Player` _asbp_third_person_character))
  (set `/Game/ThirdPerson/Blueprints/BP_ThirdPersonCharacter.NPC` self _output_get) ; Tell the player that\nthey're talking to us
  (`UserWidget.AddToViewport` (`self.W_Dialogue`) 0)
  (`self.Next Line`))

(event `self.Sphere.OnComponentEndOverlap`
  (params (OverlappedComponent :type "PrimitiveComponent Object Reference") (OtherActor :type "Actor Object Reference") (OtherComp :type "PrimitiveComponent Object Reference") (OtherBodyIndex :type Integer))
  (cast `/Game/ThirdPerson/Blueprints/BP_ThirdPersonCharacter` OtherActor)
  (`self.End Dialogue`))

(event `End Dialogue`
  (set `/Game/ThirdPerson/Blueprints/BP_ThirdPersonCharacter.NPC` null (`self.Player`)) ; Set NPC to null
  (set `self.Player` null) ; Set player to null
  (`Widget.RemoveFromParent` (`self.W_Dialogue`))
  (set `self.NextLineIndex` 0) ; Reset the index
)

(event `Next Line`
  (bind _audio (`self.Audio`))
  (bind _outrownames (`DataTableFunctionLibrary.GetDataTableRowNames` "/Game/Blueprints/DT_NPCdialogue.DT_NPCdialogue"))
  (if (> (`self.NextLineIndex`) (`KismetArrayLibrary.Array_LastIndex` _outrownames))
    (`self.End Dialogue`)
    (else
      (bind _returnvalue (`|GetDataTableRow` "/Game/Blueprints/DT_NPCdialogue.DT_NPCdialogue" (`|GetArrayItem` _outrownames (`self.NextLineIndex`)))
        (:`then`
          (`TextBlock.SetText` (`/Game/Widget/W_NPCdialogue.TextBlock_0` (`self.W_Dialogue`)) (`KismetTextLibrary.Conv_StringToText` (break `/Game/Blueprints/S_NPCdialogue` _returnvalue)))
          (`/Engine/EditorBlueprintResources/StandardMacros.IncrementInt` (`self.NextLineIndex`) ; Increment Int
            (:`  `
              (`AudioComponent.SetSound` _audio (`.VoicedLine_8_C4D5A9E1A74F11953B6E818A2B88AEF8` (break `/Game/Blueprints/S_NPCdialogue` _returnvalue)))
              (`AudioComponent.Play` _audio 0.0)
              (set `TextLayoutWidget.Justification` (select `/Game/Blueprints/E_Speaker` (`.Speaker_9_905895A7D74CF47CFCF05696C9228C44` (break `/Game/Blueprints/S_NPCdialogue` _returnvalue)) :`NewEnumerator0` "Left" :`NewEnumerator1` "Right" :`NewEnumerator2` "Center" :!type "ETextJustify Enum") (`/Game/Widget/W_NPCdialogue.TextBlock_0` (`self.W_Dialogue`))))))))))

(fn `UserConstructionScript`)